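; BP_GoldPickUp is a gold pickup that grants the top-down character a random amount of gold on overlap outside battle.
; Pickup fires once, removing its visuals, playing a coin sound, showing the amount in a screen widget, then destroying the actor.
; Its ID is added to the character's found-items array, which BeginPlay checks after a short delay to remove already-collected pickups.
; Each tick, its widget yaws toward the character's camera.
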(event `WidgetCameraFacing`
  (bind _widget (`self.Widget`))
  ;[1 1 1] WidgetCameraFacingEvent
  (`/Engine/EditorBlueprintResources/StandardMacros.IsValid` _widget
    (:`Is Valid`
      (`SceneComponent.K2_SetWorldRotation` (`self.Widget`) (`KismetMathLibrary.MakeRotator` 0.0 0.0 (.yaw (`KismetMathLibrary.FindLookAtRotation` (`SceneComponent.K2_GetComponentLocation` _widget) (`SceneComponent.K2_GetComponentLocation` (`/Game/TurnBasedTacticStarterPack/Blueprints/BP_TopDownCharacter.Camera1` (`self.Char`)))))) false false))))

(event `self.ReceiveTick`
  (params (DeltaSeconds :type "Float (single-precision)"))
  ;[1 1 1] EventTick
  (`self.WidgetCameraFacing`))

(event `self.ReceiveBeginPlay`
  ;[1 1 1] EventBeginPlay\ Check, if pick up was founded, destroy it.
  (bind _asbp_top_down_character (cast `/Game/TurnBasedTacticStarterPack/Blueprints/BP_TopDownCharacter` (`GameplayStatics.GetPlayerCharacter` 0)))
  (bind _output_get (set `self.Char` _asbp_top_down_character))
  (`KismetSystemLibrary.Delay` 0.3)
  (if (> (`KismetArrayLibrary.Array_Find` (`/Game/TurnBasedTacticStarterPack/Blueprints/BP_TopDownCharacter.Founded\\Destroyed_Items` _output_get) (`self.ID`)) -1)
    (`self.K2_DestroyActor`)))

(event `self.Box.OnComponentBeginOverlap`
  (params (OverlappedComponent :type "PrimitiveComponent Object Reference") (OtherActor :type "Actor Object Reference") (OtherComp :type "PrimitiveComponent Object Reference") (OtherBodyIndex :type Integer) (bFromSweep :type Boolean) (SweepResult :type "HitResult Structure (by ref)"))
  ;[1 1 1] Character pick up loot
  (bind _asbp_top_down_character (cast `/Game/TurnBasedTacticStarterPack/Blueprints/BP_TopDownCharacter` OtherActor))
  (if (not (`/Game/TurnBasedTacticStarterPack/Blueprints/BP_TopDownCharacter.Battle` _asbp_top_down_character))
    (`/Engine/EditorBlueprintResources/StandardMacros.DoOnce` false
      (:`Completed`
        (bind _output_get (set `self.RandomValue` (`KismetMathLibrary.RandomInteger` 100)))
        (set `/Game/TurnBasedTacticStarterPack/Blueprints/BP_TopDownCharacter.Gold` (+ (`/Game/TurnBasedTacticStarterPack/Blueprints/BP_TopDownCharacter.Gold` (`self.Char`)) _output_get) (`self.Char`))
        (`ActorComponent.K2_DestroyComponent` (`self.P_PickUp`))
        (`ActorComponent.K2_DestroyComponent` (`self.Widget`))
        (`ActorComponent.K2_DestroyComponent` (`self.Shape_Cube`))
        (`AudioComponent.Play` (`self.coins`) 0.0)
        (bind _returnvalue (`|CreateWidget` "/Game/TurnBasedTacticStarterPack/Widgets/BP_GoldImagePickUp_Widget.BP_GoldImagePickUp_Widget_C"))
        (`UserWidget.AddToViewport` _returnvalue 0)
        (`TextBlock.SetText` (`/Game/TurnBasedTacticStarterPack/Widgets/BP_GoldImagePickUp_Widget.Value` _returnvalue) (`KismetTextLibrary.Conv_IntToText` (`self.RandomValue`)))
        ;;[1 1 1] Add Pick Up to array of Founded\DestroyedItems
        (`KismetArrayLibrary.Array_Add` (`/Game/TurnBasedTacticStarterPack/Blueprints/BP_TopDownCharacter.Founded\\Destroyed_Items` (`self.Char`)) (`self.ID`))
        (`KismetSystemLibrary.Delay` 2.0)
        (`self.K2_DestroyActor`)))))

(fn `UserConstructionScript`)