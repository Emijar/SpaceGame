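; BP_GridSetup builds the tile grid for the turn-based tactics game when play begins.
; Nested loops over GridX and GridY spawn one BP_Grid actor per cell, spaced by GridSize and roughly centered on this actor's location.
; Each tile spawns regardless of collision and is stored in GridBaseArray.
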(event `self.ReceiveBeginPlay`
  (bind _grid_x (`self.Grid_X`))
  (bind _grid_y (`self.Grid_Y`))
  (bind _gridsize (`self.GridSize`))
  (bind _gridsize_2 (`self.GridSize`))
  ;[1 1 1] Build Grid
  (for _index (range 1 (+ _grid_x 1))
    (for _index_2 (range 1 (+ _grid_y 1))
      (bind _returnvalue (`|SpawnActorFromClass` "/Game/TurnBasedTacticStarterPack/Blueprints/BP_Grid.BP_Grid_C" (`KismetMathLibrary.MakeTransform` (+ (`self.K2_GetActorLocation`) (`KismetMathLibrary.MakeVector` (`KismetMathLibrary.Conv_IntToDouble` (- (* _index _gridsize) (/ (* _grid_x _gridsize_2) 2))) (`KismetMathLibrary.Conv_IntToDouble` (- (* _index_2 _gridsize) (/ (* _grid_y _gridsize_2) 2)))))) "AlwaysSpawn" "OverrideRootScale" null null))
      (`KismetArrayLibrary.Array_Add` (`self.GridBaseArray`) _returnvalue))))

(fn `UserConstructionScript`)