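; BP_BattleArea is an actor that manages one turn-based battle encounter and its enemies.
; EnemyTurn makes the enemy at the current index attack after a short delay.
; Tick checks for victory when IndexMax drops below zero, then ends battle and super armor, blends the camera back to the player, records its ID and destroys itself.
; On BeginPlay, a delayed check removes the area and enemies if that ID is already recorded.
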(event `self.ReceiveTick`
  (params (DeltaSeconds :type "Float (single-precision)"))
  ;[1 1 1] EventTick
  (`self.PlayerWin`))

(event `DoesWasDestroyed`
  ;[1 1 1] If area was destroyed earlier, this event check in array ID of this area, and, depending of that, destroy it or not.
  (`KismetSystemLibrary.Delay` 0.5)
  (if (> (`KismetArrayLibrary.Array_Find` (`/Game/TurnBasedTacticStarterPack/Blueprints/BP_TopDownCharacter.Founded\\Destroyed_Items` (`self.Char`)) (`self.ID`)) -1)
    (for _array_element (`self.Enemies Array`)
      (`/Engine/EditorBlueprintResources/StandardMacros.IsValid` _array_element
        (:`Is Valid`
          (`self.K2_DestroyActor` _array_element)
          (`self.K2_DestroyActor`)
          (set `/Game/TurnBasedTacticStarterPack/Blueprints/BP_TopDownCharacter.Battle` false (`self.Char`)))))))

(event `self.ReceiveBeginPlay`
  ;[1 1 1] Event Begin Play
  (`self.AddEnemyToArray`)
  (bind _asbp_top_down_character (cast `/Game/TurnBasedTacticStarterPack/Blueprints/BP_TopDownCharacter` (`GameplayStatics.GetPlayerCharacter` 0)))
  (set `self.Char` _asbp_top_down_character)
  (`self.DoesWasDestroyed`))

(event `AddEnemyToArray`
  ;[1 1 1] AddEnemyToArray
  (`KismetArrayLibrary.Array_Add` (`self.Enemies Array`)))

(event `EnemyTurn`
  (bind _output (`|GetArrayItem` (`self.Enemies Array`) (`self.Index`)))
  ;[1 1 1] EnemyTurn
  (`KismetSystemLibrary.Delay` 1.0)
  (`/Engine/EditorBlueprintResources/StandardMacros.IsValid` _output
    (:`Is Valid`
      (`/Game/TurnBasedTacticStarterPack/Blueprints/BP_Enemy.Attack` _output))))

(event `PlayerWin`
  (bind _char (`self.Char`))
  ;[1 1 1] EventPlayerWin
  (if (<= (`self.IndexMax`) -1)
    (`/Engine/EditorBlueprintResources/StandardMacros.DoOnce` false
      (:`Completed`
        (set `/Game/TurnBasedTacticStarterPack/Blueprints/BP_TopDownCharacter.Battle` false (`self.Char`))
        (`PlayerController.SetViewTargetWithBlend` (`GameplayStatics.GetPlayerController` 0) (`self.Char`) 2.0 "VTBlend_Linear" 0.0 false)
        (`KismetArrayLibrary.Array_Add` (`/Game/TurnBasedTacticStarterPack/Blueprints/BP_TopDownCharacter.Founded\\Destroyed_Items` (`self.Char`)) (`self.ID`))
        (set `/Game/TurnBasedTacticStarterPack/Blueprints/BP_TopDownCharacter.SuperArmorActive` false _char)
        (`SceneComponent.SetVisibility` (`/Game/TurnBasedTacticStarterPack/Blueprints/BP_TopDownCharacter.SuperArmorMesh` _char) false false)
        (`KismetSystemLibrary.Delay` 2.0)
        (`self.K2_DestroyActor`)))))

(fn `UserConstructionScript`)