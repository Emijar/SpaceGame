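; Random pickup actor for the turn-based tactics game that rewards the top-down character once when walked into outside battle.
; Chained, separately rolled RandomInteger(3) checks grant medicine, armor, gold or nothing, each with a popup widget; the ammo branch is unreachable.
; After a sound, it records its ID in the character's found-items array and destroys itself, also self-destroying on BeginPlay if already recorded.
; Its widget yaws toward the camera every tick.
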(event `WidgetCameraFacing`
  (bind _widget (`self.Widget`))
  ;[1 1 1] WidgetCameraFacingEvent
  (`/Engine/EditorBlueprintResources/StandardMacros.IsValid` _widget
    (:`Is Valid`
      (`SceneComponent.K2_SetWorldRotation` (`self.Widget`) (`KismetMathLibrary.MakeRotator` 0.0 0.0 (.yaw (`KismetMathLibrary.FindLookAtRotation` (`SceneComponent.K2_GetComponentLocation` _widget) (`SceneComponent.K2_GetComponentLocation` (`/Game/TurnBasedTacticStarterPack/Blueprints/BP_TopDownCharacter.Camera1` (`self.Char`)))))) false false))))

(event `self.ReceiveTick`
  (params (DeltaSeconds :type "Float (single-precision)"))
  ;[1 1 1] EventTick
  (`self.WidgetCameraFacing`))

(event `self.ReceiveBeginPlay`
  ;[1 1 1] Check, if pick up was founded, destroy it.
  (bind _asbp_top_down_character (cast `/Game/TurnBasedTacticStarterPack/Blueprints/BP_TopDownCharacter` (`GameplayStatics.GetPlayerCharacter` 0)))
  (bind _output_get (set `self.Char` _asbp_top_down_character))
  (`KismetSystemLibrary.Delay` 0.3)
  (if (> (`KismetArrayLibrary.Array_Find` (`/Game/TurnBasedTacticStarterPack/Blueprints/BP_TopDownCharacter.Founded\\Destroyed_Items` _output_get) (`self.ID`)) -1)
    (`self.K2_DestroyActor`)))

(event `self.Box.OnComponentBeginOverlap`
  (params (OverlappedComponent :type "PrimitiveComponent Object Reference") (OtherActor :type "Actor Object Reference") (OtherComp :type "PrimitiveComponent Object Reference") (OtherBodyIndex :type Integer) (bFromSweep :type Boolean) (SweepResult :type "HitResult Structure (by ref)"))
  ;[1 1 1] SetRandomPickUp
  (bind _asbp_top_down_character (cast `/Game/TurnBasedTacticStarterPack/Blueprints/BP_TopDownCharacter` OtherActor))
  (if (not (`/Game/TurnBasedTacticStarterPack/Blueprints/BP_TopDownCharacter.Battle` _asbp_top_down_character))
    (`/Engine/EditorBlueprintResources/StandardMacros.DoOnce` false
      (:`Completed`
        (`ActorComponent.K2_DestroyComponent` (`self.P_PickUp`))
        (`ActorComponent.K2_DestroyComponent` (`self.Widget`))
        (`ActorComponent.K2_DestroyComponent` (`self.Shape_Cube`))
        (if (== (`KismetMathLibrary.RandomInteger` 3) 0)
          (set `/Game/TurnBasedTacticStarterPack/Blueprints/BP_TopDownCharacter.Medicine` (+ (`/Game/TurnBasedTacticStarterPack/Blueprints/BP_TopDownCharacter.Medicine` (`self.Char`)) 1) (`self.Char`))
          (bind _returnvalue (`|CreateWidget` "/Game/TurnBasedTacticStarterPack/Widgets/BP_MedicinePickUpImage_Widget.BP_MedicinePickUpImage_Widget_C"))
          (`UserWidget.AddToViewport` _returnvalue 0)
          (`TextBlock.SetText` (`/Game/TurnBasedTacticStarterPack/Widgets/BP_MedicinePickUpImage_Widget.Value` _returnvalue) "1")
          (`/Engine/EditorBlueprintResources/StandardMacros.IsValid` _returnvalue
            (:`Is Valid`
              _))
          (elif (== (`KismetMathLibrary.RandomInteger` 3) 1)
            (set `/Game/TurnBasedTacticStarterPack/Blueprints/BP_TopDownCharacter.Armor` (+ (`/Game/TurnBasedTacticStarterPack/Blueprints/BP_TopDownCharacter.Armor` (`self.Char`)) 25.0) (`self.Char`))
            (bind _returnvalue_2 (`|CreateWidget` "/Game/TurnBasedTacticStarterPack/Widgets/BP_ArmorPickUpImage_Widget.BP_ArmorPickUpImage_Widget_C"))
            (`UserWidget.AddToViewport` _returnvalue_2 0)
            (`TextBlock.SetText` (`/Game/TurnBasedTacticStarterPack/Widgets/BP_ArmorPickUpImage_Widget.Value` _returnvalue_2) "25")
            (`/Engine/EditorBlueprintResources/StandardMacros.IsValid` _returnvalue_2
              (:`Is Valid`
                _))
            (elif (== (`KismetMathLibrary.RandomInteger` 3) 2)
              (bind _output_get (set `self.RandomGold` (`KismetMathLibrary.RandomInteger` 100)))
              (set `/Game/TurnBasedTacticStarterPack/Blueprints/BP_TopDownCharacter.Gold` (+ (`/Game/TurnBasedTacticStarterPack/Blueprints/BP_TopDownCharacter.Gold` (`self.Char`)) _output_get) (`self.Char`))
              (bind _returnvalue_3 (`|CreateWidget` "/Game/TurnBasedTacticStarterPack/Widgets/BP_GoldImagePickUp_Widget.BP_GoldImagePickUp_Widget_C"))
              (`UserWidget.AddToViewport` _returnvalue_3 0)
              (`TextBlock.SetText` (`/Game/TurnBasedTacticStarterPack/Widgets/BP_GoldImagePickUp_Widget.Value` _returnvalue_3) (`KismetTextLibrary.Conv_IntToText` (`self.RandomGold`)))
              (`/Engine/EditorBlueprintResources/StandardMacros.IsValid` _returnvalue_3
                (:`Is Valid`
                  _))
              (elif (== (`KismetMathLibrary.RandomInteger` 3) 3)
                (bind _output_get_2 (set `self.RandomAmmo` (`KismetMathLibrary.RandomInteger` 10)))
                (set `/Game/TurnBasedTacticStarterPack/Blueprints/BP_TopDownCharacter.MaxAmmo` (+ (`/Game/TurnBasedTacticStarterPack/Blueprints/BP_TopDownCharacter.MaxAmmo` (`self.Char`)) _output_get_2) (`self.Char`))
                (bind _returnvalue_4 (`|CreateWidget` "/Game/TurnBasedTacticStarterPack/Widgets/BP_AmmoImagePIckUp_Widget.BP_AmmoImagePIckUp_Widget_C"))
                (`UserWidget.AddToViewport` _returnvalue_4 0)
                (`TextBlock.SetText` (`/Game/TurnBasedTacticStarterPack/Widgets/BP_AmmoImagePIckUp_Widget.Value` _returnvalue_4) (`KismetTextLibrary.Conv_IntToText` (`self.RandomAmmo`)))
                (`/Engine/EditorBlueprintResources/StandardMacros.IsValid` _returnvalue_4
                  (:`Is Valid`
                    _))
                (else
                  (bind _returnvalue_5 (`|CreateWidget` "/Game/TurnBasedTacticStarterPack/Widgets/BP_EmptyPickUp-Widget.BP_EmptyPickUp-Widget_C"))
                  (`UserWidget.AddToViewport` _returnvalue_5 0)
                  (`/Engine/EditorBlueprintResources/StandardMacros.IsValid` _returnvalue_5
                    (:`Is Valid`
                      _)))))))
        (`AudioComponent.Play` (`self.PickUpSound`) 0.0)
        ;;[1 1 1] Add Pick Up to array of Founded\DestroyedItems
        (`KismetArrayLibrary.Array_Add` (`/Game/TurnBasedTacticStarterPack/Blueprints/BP_TopDownCharacter.Founded\\Destroyed_Items` (`self.Char`)) (`self.ID`))
        (`KismetSystemLibrary.Delay` 2.0)
        (`self.K2_DestroyActor`)))))

(fn `UserConstructionScript`)