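; Enemy unit for turn-based tactics combat that shoots or approaches the player on its turn.
; Attack handles frozen turn skips, rolls distance-based hit odds and line-traces, leading to firing, missing, reloading or moving toward the player.
; EndTurn advances the BattleArea index to the next enemy or returns control to the player.
; Also manages armor and health damage, camera-facing health and hover hit-chance widgets, and removal from the battle on death.
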(event `EnemyFire`
  (bind _mesh (`self.Mesh`))
  ;[1 1 1] Enemy Fire
  (`SkeletalMeshComponent.PlayAnimation` (`self.Mesh`) "/Game/TurnBasedTacticStarterPack/ExampleContent/AnimStarterPack/Fire_Shotgun_Hip.Fire_Shotgun_Hip" false)
  ;;[1 0.8179 0.01812] If ammo not enough, reload
  (if (>= (`self.Ammo`) 1)
    (set `self.Ammo` (- (`self.Ammo`) 1))
    (`ActorComponent.SetActive` (`self.P_Explosion`) true false)
    ;;[1 0 0.6115] If SuperArmorActive variable false, apply damage to player.
    (if (not (`/Game/TurnBasedTacticStarterPack/Blueprints/BP_TopDownCharacter.SuperArmorActive` (`self.Char`)))
      (`GameplayStatics.ApplyDamage` (`self.Char`) (`self.Damage`))
      (`GameplayStatics.SpawnEmitterAtLocation` "/Game/TurnBasedTacticStarterPack/ExampleContent/StarterContent/Particles/P_Explosion.P_Explosion" (`self.K2_GetActorLocation` (`self.Char`))))
    (`AudioComponent.Play` (`self.Audio`) 0.0)
    (`KismetSystemLibrary.Delay` 1.0)
    (`/Engine/EditorBlueprintResources/StandardMacros.IsValid` _mesh
      (:`Is Valid`
        (`SkeletalMeshComponent.PlayAnimation` _mesh "/Game/TurnBasedTacticStarterPack/ExampleContent/AnimStarterPack/Idle_Rifle_Hip.Idle_Rifle_Hip" true)))
    (else
      (`self.Reloadig`))))

(event `self.ReceiveBeginPlay`
  ;[1 1 1] Event Begin Play.
  (bind _asbp_top_down_controller (cast `/Game/TurnBasedTacticStarterPack/Blueprints/BP_TopDownController` (`GameplayStatics.GetPlayerController` 0)))
  (set `self.PlayerController` _asbp_top_down_controller)
  (bind _asbp_top_down_character (cast `/Game/TurnBasedTacticStarterPack/Blueprints/BP_TopDownCharacter` (`GameplayStatics.GetPlayerCharacter` 0)))
  (set `self.Char` _asbp_top_down_character)
  (`SkeletalMeshComponent.PlayAnimation` (`self.Mesh`) "/Game/TurnBasedTacticStarterPack/ExampleContent/AnimStarterPack/Idle_Rifle_Hip.Idle_Rifle_Hip" true)
  ;;[0.06104 1 0] Set random ammo and max ammo values
  (set `self.Ammo` (`KismetMathLibrary.RandomInteger` 5))
  (set `self.MaxAmmo` (`KismetMathLibrary.RandomInteger` 40)))

(event `self.ReceiveTick`
  (params (DeltaSeconds :type "Float (single-precision)"))
  ;[1 1 1] Event Tick
  (`self.EnemyHealthWidgetEvent`)
  (`self.HealthWidgetCameraFacing`)
  (`self.Hit Probability WidgetCameraFacing`)
  (if (<= (`self.Health`) 0.0)
    (`/Engine/EditorBlueprintResources/StandardMacros.DoOnce` false
      (:`Completed`
        (`self.Death`)))))

(event `ShotPast`
  ;[1 1 1] ShotPast
  (`/Game/TurnBasedTacticStarterPack/Blueprints/BP_TopDownCharacter.ShotPastWidgetEvent` (`self.Char`))
  (`SkeletalMeshComponent.PlayAnimation` (`self.Mesh`) "/Game/TurnBasedTacticStarterPack/ExampleContent/AnimStarterPack/Fire_Shotgun_Hip.Fire_Shotgun_Hip" false)
  (`ActorComponent.SetActive` (`self.P_Explosion`) true false)
  (`KismetSystemLibrary.Delay` 0.5)
  (`AudioComponent.Play` (`self.Audio`) 0.0)
  (`KismetSystemLibrary.Delay` 0.5)
  (`SkeletalMeshComponent.PlayAnimation` (`self.Mesh`) "/Game/TurnBasedTacticStarterPack/ExampleContent/AnimStarterPack/Idle_Rifle_Hip.Idle_Rifle_Hip" true)
  (`self.EndTurn`))

(event `SearchPoint`
  ;[1 1 1] Search Point. Of enemy far to player, he will come closer.
  (`SkeletalMeshComponent.PlayAnimation` (`self.Mesh`) "/Game/TurnBasedTacticStarterPack/ExampleContent/AnimStarterPack/Walk_Fwd_Rifle_Ironsights.Walk_Fwd_Rifle_Ironsights" true)
  (`AIBlueprintHelperLibrary.SimpleMoveToLocation` (`self.GetController`) (+ (/ (`self.K2_GetActorLocation`) 2.0) (/ (`self.K2_GetActorLocation` (`self.Char`)) 2.0)))
  (`KismetSystemLibrary.Delay` 1.25)
  (`SkeletalMeshComponent.PlayAnimation` (`self.Mesh`) "/Game/TurnBasedTacticStarterPack/ExampleContent/AnimStarterPack/Idle_Rifle_Hip.Idle_Rifle_Hip" true)
  (`KismetSystemLibrary.Delay` 1.0)
  (`self.EndTurn`))

(event `Attack`
  (bind _distance (`self.Distance`))
  (bind _frozenturnindex (`self.FrozenTurnIndex`))
  ;[1 1 1] Attack
  (if (`self.Frozen `)
    ;;[0.01415 0.3663 1] If unit already skips to turns. variable "Frozen" set to false
    (if (< _frozenturnindex 2)
      ;;[0 0.211 1] If variable "Frozen" true, unit skips to turns
      (set `self.FrozenTurnIndex` (+ _frozenturnindex 1))
      (`self.EndTurn`)
      (else
        (set `self.Frozen ` false)
        (`PrimitiveComponent.SetMaterial` (`self.Mesh`) 0 "/Game/TurnBasedTacticStarterPack/ExampleContent/AnimStarterPack/UE4_Mannequin/Materials/M_UE4Man_BodyEnemy.M_UE4Man_BodyEnemy")
        (set `self.FrozenTurnIndex` 0)
        (`self.K2_SetActorRotation` (`KismetMathLibrary.MakeRotator` 0.0 0.0 (.yaw (`KismetMathLibrary.FindLookAtRotation` (`self.K2_GetActorLocation`) (`self.K2_GetActorLocation` (`self.Char`))))) :!label _label)
        (set `self.Distance` (`KismetMathLibrary.VSize` (- (`self.K2_GetActorLocation`) (`self.K2_GetActorLocation` (`self.Char`)))))
        (if (<= (`self.Distance`) 500.0)
          (`KismetSystemLibrary.PrintString` "90%")
          (if (`KismetMathLibrary.RandomBoolWithWeight` 0.9)
            (bind _outhit (`KismetSystemLibrary.LineTraceSingle` :`Start` (`self.K2_GetActorLocation`) :`End` (`self.K2_GetActorLocation` (`self.Char`)) :`TraceChannel` "TraceTypeQuery2" :`bTraceComplex` true :`DrawDebugType` "ForDuration" :`DrawTime` 1.0 :!label _label_2))
            (if (== (`.HitActor` (`GameplayStatics.BreakHitResult` _outhit)) (`self.Char`))
              (`self.EnemyFire`)
              (`self.EndTurn`)
              (else
                (`self.SearchPoint`)
                (`self.EndTurn`)))
            (else
              (`self.ShotPast`)))
          (elif (<= (`self.Distance`) 750.0)
            (`KismetSystemLibrary.PrintString` "70%")
            (if (`KismetMathLibrary.RandomBoolWithWeight` 0.7)
              (goto _label_2)
              (else
                (`self.ShotPast`)))
            (else
              (`KismetSystemLibrary.PrintString` (`KismetStringLibrary.Conv_DoubleToString` _distance))
              (if (<= _distance 1000.0)
                (`KismetSystemLibrary.PrintString` "50%")
                (if (`KismetMathLibrary.RandomBoolWithWeight` 0.5)
                  (goto _label_2)
                  (else
                    (`self.ShotPast`)))
                (else
                  (`KismetSystemLibrary.PrintString` "To far" true true (struct :`R` 1.0 :`G` 0.013839 :`A` 1.0))
                  (`self.SearchPoint`))))))))
    (else
      (goto _label))))

(event `EndTurn`
  (bind _battlearea (`/Game/TurnBasedTacticStarterPack/Blueprints/BP_TopDownCharacter.BattleArea` (`self.Char`)))
  (bind _battlearea_2 (`/Game/TurnBasedTacticStarterPack/Blueprints/BP_TopDownCharacter.BattleArea` (`self.Char`)))
  ;[1 1 1] End Enemy Turn.  In BP_Battle Area we have Index and Index Max variebles. Battle start from 0 index, then, after enemy turn, we plus 1 to index. After that, if index not equal Index Max, enemy made next turn, but if already Index = Index Max, then turn player and set index to zero. If players dead, we subtract from Index Max.
  (`KismetSystemLibrary.Delay` 0.5)
  (if (< (`/Game/TurnBasedTacticStarterPack/Blueprints/BP_BattleArea.Index` _battlearea) (`/Game/TurnBasedTacticStarterPack/Blueprints/BP_BattleArea.IndexMax` _battlearea))
    (set `/Game/TurnBasedTacticStarterPack/Blueprints/BP_BattleArea.Index` (+ (`/Game/TurnBasedTacticStarterPack/Blueprints/BP_BattleArea.Index` _battlearea_2) 1) _battlearea_2)
    (`/Game/TurnBasedTacticStarterPack/Blueprints/BP_BattleArea.EnemyTurn` (`/Game/TurnBasedTacticStarterPack/Blueprints/BP_TopDownCharacter.BattleArea` (`self.Char`)))
    (`KismetSystemLibrary.PrintString` "NextEnemyTurn")
    (`self.DestroyGrid`)
    (else
      ;;[0 1 0.1405] If all enemy units made their turn, then the player's turn
      (set `/Game/TurnBasedTacticStarterPack/Blueprints/BP_TopDownController.TunrOver` false (`self.PlayerController`))
      (set `/Game/TurnBasedTacticStarterPack/Blueprints/BP_BattleArea.Index` 0 (`/Game/TurnBasedTacticStarterPack/Blueprints/BP_TopDownCharacter.BattleArea` (`self.Char`)))
      (`/Game/TurnBasedTacticStarterPack/Blueprints/BP_TopDownCharacter.ResetCheck` (`self.Char`))
      (`self.DestroyGrid`)
      (`/Game/TurnBasedTacticStarterPack/Blueprints/BP_TopDownCharacter.SpawnGrid` (`self.Char`)))))

(event `Reloadig`
  (bind _mesh (`self.Mesh`))
  (bind _maxammo (`self.MaxAmmo`))
  (bind _needammo (`self.NeedAmmo`))
  ;[1 1 1] Reloading
  (`KismetSystemLibrary.PrintString` "reloading")
  (if (< (`self.Ammo`) 5)
    (if (>= (`self.MaxAmmo`) 1)
      (set `self.NeedAmmo` (- 5 (`self.Ammo`)))
      (if (<= _maxammo _needammo)
        (set `self.Ammo` (+ (`self.Ammo`) (`self.MaxAmmo`)))
        (set `self.MaxAmmo` 0)
        (else
          (set `self.MaxAmmo` (- _maxammo _needammo))
          (set `self.Ammo` 5)))
      (`SkeletalMeshComponent.PlayAnimation` (`self.Mesh`) "/Game/TurnBasedTacticStarterPack/ExampleContent/AnimStarterPack/Reload_Shotgun_Hip.Reload_Shotgun_Hip" false)
      (`AudioComponent.Play` (`self.RobotVoice_Reload_wav`) 0.0)
      (`self.EndTurn`)
      (`AudioComponent.Play` (`self.ReloadSound`) 0.0)
      (`KismetSystemLibrary.Delay` 1.5)
      (`/Engine/EditorBlueprintResources/StandardMacros.IsValid` _mesh
        (:`Is Valid`
          (`SkeletalMeshComponent.PlayAnimation` _mesh "/Game/TurnBasedTacticStarterPack/ExampleContent/AnimStarterPack/Idle_Rifle_Hip.Idle_Rifle_Hip" true)))
      (else
        (`AudioComponent.Play` (`self.NeedAmmo_Cue`) 0.0)))))

(event `EnemyHealthWidgetEvent`
  ;[1 1 1] Enemy Health Widget Event
  (if (> (`self.Health`) 0.0)
    (bind _asbp_enemy_health_widget (cast `/Game/TurnBasedTacticStarterPack/Widgets/BP_EnemyHealth_Widget` (`WidgetComponent.GetUserWidgetObject` (`self.HealthWidget`))))
    (set `self.EnemyWidget` _asbp_enemy_health_widget)
    (`TextBlock.SetText` (`/Game/TurnBasedTacticStarterPack/Widgets/BP_EnemyHealth_Widget.EnemyHealthText` (`self.EnemyWidget`)) (`KismetTextLibrary.Conv_DoubleToText` (`self.Health`) "HalfToEven"))
    (`TextBlock.SetText` (`/Game/TurnBasedTacticStarterPack/Widgets/BP_EnemyHealth_Widget.EnemyArmorText` (`self.EnemyWidget`)) (`KismetTextLibrary.Conv_DoubleToText` (`self.Armor`) "HalfToEven"))))

(event `self.CapsuleComponent.OnBeginCursorOver`
  (params (TouchedComponent :type "PrimitiveComponent Object Reference"))
  (bind _distance (`self.Distance`))
  ;[1 1 1] When cursor over enemy, shows hit probability depending on distance between player and enemy
  (set `self.Distance` (`KismetMathLibrary.VSize` (- (`self.K2_GetActorLocation`) (`self.K2_GetActorLocation` (`self.Char`)))))
  (if (<= (`self.Distance`) 500.0)
    (`KismetSystemLibrary.PrintString` "90%" true true (struct :`R` 1.0 :`G` 0.117631 :`A` 1.0))
    (bind _asbp_hit_probability_widget (cast `/Game/TurnBasedTacticStarterPack/Widgets/BP_Hit_Probability_Widget` (`WidgetComponent.GetUserWidgetObject` (`self.HitProbability Widget`))))
    (`TextBlock.SetText` (`/Game/TurnBasedTacticStarterPack/Widgets/BP_Hit_Probability_Widget.Percentage` _asbp_hit_probability_widget) "90%")
    (elif (<= (`self.Distance`) 750.0)
      (`KismetSystemLibrary.PrintString` "70%" true true (struct :`R` 1.0 :`G` 0.21838 :`A` 1.0))
      (bind _asbp_hit_probability_widget_2 (cast `/Game/TurnBasedTacticStarterPack/Widgets/BP_Hit_Probability_Widget` (`WidgetComponent.GetUserWidgetObject` (`self.HitProbability Widget`))))
      (`TextBlock.SetText` (`/Game/TurnBasedTacticStarterPack/Widgets/BP_Hit_Probability_Widget.Percentage` _asbp_hit_probability_widget_2) "70%")
      (else
        (`KismetSystemLibrary.PrintString` (`KismetStringLibrary.Conv_DoubleToString` _distance))
        (if (<= _distance 1000.0)
          (`KismetSystemLibrary.PrintString` "50%" true true (struct :`R` 1.0 :`G` 0.199368 :`A` 1.0))
          (bind _asbp_hit_probability_widget_3 (cast `/Game/TurnBasedTacticStarterPack/Widgets/BP_Hit_Probability_Widget` (`WidgetComponent.GetUserWidgetObject` (`self.HitProbability Widget`))))
          (`TextBlock.SetText` (`/Game/TurnBasedTacticStarterPack/Widgets/BP_Hit_Probability_Widget.Percentage` _asbp_hit_probability_widget_3) "50%")
          (else
            (`KismetSystemLibrary.PrintString` "To far")
            (bind _asbp_hit_probability_widget_4 (cast `/Game/TurnBasedTacticStarterPack/Widgets/BP_Hit_Probability_Widget` (`WidgetComponent.GetUserWidgetObject` (`self.HitProbability Widget`))))
            (`TextBlock.SetText` (`/Game/TurnBasedTacticStarterPack/Widgets/BP_Hit_Probability_Widget.Percentage` _asbp_hit_probability_widget_4) "ToFar"))))))
  (`SceneComponent.SetVisibility` (`self.HitProbability Widget`) true false))

(event `self.ReceiveAnyDamage`
  (params (Damage :type "Float (single-precision)") (DamageType :type "DamageType Object Reference") (InstigatedBy :type "Controller Object Reference") (DamageCauser :type "Actor Object Reference"))
  (bind _mesh (`self.Mesh`))
  ;[1 1 1] Event Take Any Damage.
  (`SkeletalMeshComponent.PlayAnimation` (`self.Mesh`) "/Game/TurnBasedTacticStarterPack/ExampleContent/AnimStarterPack/Hit_React_1.Hit_React_1" false)
  (if (>= (`self.Armor`) 50.0)
    (bind _output_get (set `self.Armor` (- (`self.Armor`) Damage)))
    (if (< _output_get 0.0)
      (set `self.Armor` 0.0)
      (set `self.Health` (- (`self.Health`) Damage) :!label _label_3))
    (else
      (goto _label_3)))
  (`KismetSystemLibrary.Delay` 1.0)
  (`/Engine/EditorBlueprintResources/StandardMacros.IsValid` _mesh
    (:`Is Valid`
      (`SkeletalMeshComponent.PlayAnimation` _mesh "/Game/TurnBasedTacticStarterPack/ExampleContent/AnimStarterPack/Idle_Rifle_Hip.Idle_Rifle_Hip" true))))

(event `self.CapsuleComponent.OnEndCursorOver`
  (params (TouchedComponent :type "PrimitiveComponent Object Reference"))
  ;[1 1 1] When cursor over enemy, shows hit probability depending on distance between player and enemy
  (`SceneComponent.SetVisibility` (`self.HitProbability Widget`) false false))

(event `DestroyGrid`
  ;[1 1 1] DestroyGridEvent
  (bind _outactors (`GameplayStatics.GetAllActorsOfClass` "/Game/TurnBasedTacticStarterPack/Blueprints/BP_Grid.BP_Grid_C"))
  (for _array_element _outactors
    (`self.K2_DestroyActor` _array_element)))

(event `HealthWidgetCameraFacing`
  (bind _healthwidget (`self.HealthWidget`))
  (bind _char (`self.Char`))
  (bind _healthwidget_2 (`self.HealthWidget`))
  ;[1 1 1] HealthWidgetCameraFacingEvent.
  (if (`/Game/TurnBasedTacticStarterPack/Blueprints/BP_TopDownCharacter.Battle` _char)
    (`/Engine/EditorBlueprintResources/StandardMacros.IsValid` _healthwidget
      (:`Is Valid`
        (`SceneComponent.K2_SetWorldRotation` (`self.HealthWidget`) (`KismetMathLibrary.MakeRotator` 0.0 0.0 (.yaw (`KismetMathLibrary.FindLookAtRotation` (`SceneComponent.K2_GetComponentLocation` _healthwidget) (`SceneComponent.K2_GetComponentLocation` (`/Game/TurnBasedTacticStarterPack/Blueprints/BP_BattleArea.Camera` (`/Game/TurnBasedTacticStarterPack/Blueprints/BP_TopDownCharacter.BattleArea` _char)))))) false false)))
    (else
      (`/Engine/EditorBlueprintResources/StandardMacros.IsValid` _healthwidget_2
        (:`Is Valid`
          (`SceneComponent.K2_SetWorldRotation` (`self.HealthWidget`) (`KismetMathLibrary.MakeRotator` 0.0 0.0 (.yaw (`KismetMathLibrary.FindLookAtRotation` (`SceneComponent.K2_GetComponentLocation` _healthwidget_2) (`SceneComponent.K2_GetComponentLocation` (`/Game/TurnBasedTacticStarterPack/Blueprints/BP_TopDownCharacter.Camera1` (`self.Char`)))))) false false))))))

(event `Hit Probability WidgetCameraFacing`
  (bind _healthwidget (`self.HealthWidget`))
  (bind _char (`self.Char`))
  ;[1 1 1] HitProbabilityWidgetCameraFacingEvent
  (if (`/Game/TurnBasedTacticStarterPack/Blueprints/BP_TopDownCharacter.Battle` _char)
    (`/Engine/EditorBlueprintResources/StandardMacros.IsValid` _healthwidget
      (:`Is Valid`
        (`SceneComponent.K2_SetWorldRotation` (`self.HitProbability Widget`) (`KismetMathLibrary.MakeRotator` 0.0 0.0 (.yaw (`KismetMathLibrary.FindLookAtRotation` (`SceneComponent.K2_GetComponentLocation` _healthwidget) (`SceneComponent.K2_GetComponentLocation` (`/Game/TurnBasedTacticStarterPack/Blueprints/BP_BattleArea.Camera` (`/Game/TurnBasedTacticStarterPack/Blueprints/BP_TopDownCharacter.BattleArea` _char)))))) false false)))))

(event `Death`
  (bind _battlearea (`/Game/TurnBasedTacticStarterPack/Blueprints/BP_TopDownCharacter.BattleArea` (`self.Char`)))
  ;[1 1 1] Death event. Removin unit from array and - 1 from Index Max in Battle Area
  (`KismetArrayLibrary.Array_RemoveItem` (`/Game/TurnBasedTacticStarterPack/Blueprints/BP_BattleArea.Enemies Array` (`/Game/TurnBasedTacticStarterPack/Blueprints/BP_TopDownCharacter.BattleArea` (`self.Char`))) self)
  (set `/Game/TurnBasedTacticStarterPack/Blueprints/BP_BattleArea.IndexMax` (- (`/Game/TurnBasedTacticStarterPack/Blueprints/BP_BattleArea.IndexMax` _battlearea) 1) _battlearea)
  (`SceneComponent.SetVisibility` (`self.Mesh`) false false)
  (`ActorComponent.K2_DestroyComponent` (`self.HealthWidget`))
  (`ActorComponent.K2_DestroyComponent` (`self.CapsuleComponent`))
  (`ActorComponent.K2_DestroyComponent` (`self.Mesh`))
  (`ActorComponent.K2_DestroyComponent` (`self.HitProbability Widget`))
  (`ActorComponent.K2_DestroyComponent` (`self.SK_FPGun`)))

(fn `UserConstructionScript`
  (`SceneComponent.K2_AttachToComponent` (`self.SK_FPGun`) (`self.Mesh`) "hand_rSocket" "SnapToTarget" "SnapToTarget" "SnapToTarget" true))